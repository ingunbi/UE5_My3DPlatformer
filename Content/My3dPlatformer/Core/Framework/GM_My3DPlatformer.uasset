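; Game mode for a 3D platformer that tracks the respawn point and handles winning.
; BeginPlay seeds the respawn transform from a PlayerStart.
; UpdateRespawnPoint returns any current checkpoint to normal, even if re-triggered, then stores a different checkpoint and its transform with a sound.
; WinTheGame prints a victory message and makes BP_MainCharacter enter its celebration.
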(event `self.ReceiveBeginPlay`
  (bind _returnvalue (`GameplayStatics.GetActorOfClass` "/Script/Engine.PlayerStart"))
  (set `self.RespawnPoint` (`self.GetTransform` _returnvalue)))

(event `WinTheGame`
  (`KismetSystemLibrary.PrintString` "You Win!!!!")
  (bind _asbp_main_character (cast `/Game/My3dPlatformer/Core/Player/BP_MainCharacter` (`GameplayStatics.GetPlayerCharacter` 0)))
  (`/Game/My3dPlatformer/Core/Player/BP_MainCharacter.EnterCelebration` _asbp_main_character))

(fn `Update Respawn Point`
  (params (NewRespawnPoint :type "Transform Structure") (`NewCheckpoint Ref` :type "/Game/My3dPlatformer/Core/RespwanSystem/BP_CheckPoint Object Reference"))
  (bind _currentcheckpoint_ref (`self.CurrentCheckpoint Ref`))
  (`|ExecutionSequence`
    (:`then_0`
      (if (`KismetSystemLibrary.IsValid` _currentcheckpoint_ref)
        (`/Game/My3dPlatformer/Core/RespwanSystem/BP_CheckPoint.ReturnToNormal` _currentcheckpoint_ref)))
    (:`then_1`
      (if (not (== `NewCheckpoint Ref` (`self.CurrentCheckpoint Ref`)))
        (set `self.RespawnPoint` (`local.NewRespawnPoint`))
        (set `self.CurrentCheckpoint Ref` (`local.NewCheckpoint Ref`))
        (`GameplayStatics.PlaySound2D` "/Game/Hour_of_Code/Audio/SFX_checkpoint.SFX_checkpoint" 1.0 1.0 0.0 null null)))))

(fn `UserConstructionScript`)